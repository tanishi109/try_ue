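; Player character with camera-relative walking, sprinting and look controls, which carries a coin count and can pick up a scroll to clear the game.
; A looping timer drops a coin whenever horizontal speed reaches sprint speed, spawning a physics pickup flung in a random horizontal direction.
; Any damage kills once: the body ragdolls, all coins scatter and a death effect plays.
; Obtaining the scroll stops movement and prints a clear message after a delay.
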(event `self.ReceiveBeginPlay`
  (set `CharacterMovementComponent.MaxWalkSpeed` (`self.GroundWalkSpeed`) (`self.CharacterMovement`))
  (`KismetSystemLibrary.K2_SetTimer` null "CheckSprintRisk" 0.5 true))

(event `InputAxis|MoveForward`
  (params (AxisValue :type "Float (single-precision)"))
  (`self.AddMovementInput` (`/Game/BluePrints/PNFuncLibrary.FlattenDirection` (`SceneComponent.GetForwardVector` (`self.Camera`))) AxisValue))

(event `InputAxis|MoveRight`
  (params (AxisValue :type "Float (single-precision)"))
  (`self.AddMovementInput` (`/Game/BluePrints/PNFuncLibrary.FlattenDirection` (`SceneComponent.GetRightVector` (`self.Camera`))) AxisValue))

(event `InputAction|Sprint`
  (params (Key :type "Key Structure"))
  (bind _charactermovement (`self.CharacterMovement`))
  (:`Pressed`
    (set `CharacterMovementComponent.MaxWalkSpeed` (`self.GroundSprintSpeed`) _charactermovement))
  (:`Released`
    (set `CharacterMovementComponent.MaxWalkSpeed` (`self.GroundWalkSpeed`) _charactermovement)))

(event `InputAxis|LookCameraUp`
  (params (AxisValue :type "Float (single-precision)"))
  (`self.AddControllerPitchInput` AxisValue))

(event `InputAxis|LookCameraRight`
  (params (AxisValue :type "Float (single-precision)"))
  (`self.AddControllerYawInput` AxisValue))

(event `self.ReceiveAnyDamage`
  (params (Damage :type "Float (single-precision)") (DamageType :type "DamageType Object Reference") (InstigatedBy :type "Controller Object Reference") (DamageCauser :type "Actor Object Reference"))
  (bind _mesh (`self.Mesh`))
  (`/Engine/EditorBlueprintResources/StandardMacros.DoOnce` false
    (:`Completed`
      (`|ExecutionSequence`
        (:`then_0`
          (`KismetSystemLibrary.PrintString` "Died!")
          (`CharacterMovementComponent.DisableMovement` (`self.CharacterMovement`))
          (`self.SetLifeSpan` 5.0)
          (`PrimitiveComponent.SetCollisionProfileName` _mesh "Ragdoll")
          (`PrimitiveComponent.SetSimulatePhysics` _mesh true))
        (:`then_1`
          (`self.DropAllCoins`))
        (:`then_2`
          (`ActorComponent.Activate` (`self.DeathFx`) false))))))

(event `ObtainScroll`
  (`CharacterMovementComponent.DisableMovement` (`self.CharacterMovement`))
  (set `self.HasScroll` true)
  (`KismetSystemLibrary.Delay` 5.0)
  (`KismetSystemLibrary.PrintString` "Clear!"))

(event `DropAllCoins`
  (while (> (`self.NumOfCoins`) 0)
    (`self.DropCoin` 1)))

(fn `AddCoin`
  (params (Num :type Integer :default 1))
  (set `self.NumOfCoins` (+ (`self.NumOfCoins`) Num)))

(fn `CheckSprintRisk`
  (if (>= (`/Game/BluePrints/PNActorMacroLibrary.GetFlatSpeed`) (`self.GroundSprintSpeed`))
    (`self.DropCoin` 1)))

(fn `DropCoin`
  (params (Num :type Integer :default 1))
  (bind _returnvalue (- (`self.NumOfCoins`) Num))
  (if (>= _returnvalue 0)
    (set `self.NumOfCoins` _returnvalue)
    (bind _returnvalue_2 (`|SpawnActorFromClass` "/Game/BluePrints/PNPickupCoinActor.PNPickupCoinActor_C" (`SceneComponent.GetSocketTransform` (`self.Mesh`) "CoinSpawnPoint" "RTS_World") "Undefined" "OverrideRootScale" null null))
    (bind _staticmeshcomponent (`StaticMeshActor.StaticMeshComponent` _returnvalue_2))
    (`PrimitiveComponent.SetSimulatePhysics` _staticmeshcomponent true)
    (`PrimitiveComponent.AddImpulse` _staticmeshcomponent (`KismetMathLibrary.RotateAngleAxis` (`KismetMathLibrary.MakeVector` 200.0) (`KismetMathLibrary.RandomFloatInRange` 0.0 360.0) (0.0 0.0 1.0)) "None" true)
    (else
      (set `self.NumOfCoins` 0))))

(fn `GetNumOfCoins`
  (returns (NewParam :type Integer))
  (return (`self.NumOfCoins`)))

(fn `UserConstructionScript`)