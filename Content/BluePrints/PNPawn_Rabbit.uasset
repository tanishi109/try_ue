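; Rabbit character that damages whatever it touches and can switch between walking and sprinting.
; Overlapping any actor deals heavy damage, and while sprinting a short forward trace from the spine socket each tick damages whatever blocks it.
; BeginSprint and EndSprint set walk speed and the sprint flag.
; CanSeePlayerPawn uses a single debug-drawn forward line trace to report whether the hit actor has the Player tag.
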(event `self.ReceiveBeginPlay`
  (set `CharacterMovementComponent.MaxWalkSpeed` (`self.WalkGroundSpeed`) (`self.CharacterMovement`)))

(event `self.ReceiveActorBeginOverlap`
  (params (OtherActor :type "Actor Object Reference"))
  (`GameplayStatics.ApplyDamage` OtherActor 100.0))

(event `self.ReceiveTick`
  (params (DeltaSeconds :type "Float (single-precision)"))
  (bind _returnvalue (`SceneComponent.GetSocketLocation` (`self.Mesh`) "spine"))
  (if (`self.IsSprint`)
    (bind _outhit (`KismetSystemLibrary.LineTraceSingle` _returnvalue (+ _returnvalue (* (`self.GetActorForwardVector`) 50)) "TraceTypeQuery3"))
    (bind (_bblockinghit _binitialoverlap _time _distance _location _impactpoint _normal _impactnormal _physmat _hitactor) (`GameplayStatics.BreakHitResult` _outhit))
    (if _bblockinghit
      (`GameplayStatics.ApplyDamage` _hitactor 100.0))))

(fn `BeginSprint`
  (set `CharacterMovementComponent.MaxWalkSpeed` (`self.SprintGroundSpeed`) (`self.CharacterMovement`))
  (set `self.IsSprint` true))

(fn `CanSeePlayerPawn`
  (returns (CanSee :type Boolean) (SeenActor :type "Actor Object Reference"))
  (bind _returnvalue (`self.K2_GetActorLocation`))
  (bind _outhit (`KismetSystemLibrary.LineTraceSingle` :`Start` _returnvalue :`End` (+ _returnvalue (* (`self.GetActorForwardVector`) (`self.SightLength`))) :`TraceChannel` "TraceTypeQuery3" :`DrawDebugType` "ForOneFrame"))
  (bind (_bblockinghit _binitialoverlap _time _distance _location _impactpoint _normal _impactnormal _physmat _hitactor) (`GameplayStatics.BreakHitResult` _outhit))
  (if (`KismetSystemLibrary.IsValid` _hitactor)
    (return (`self.ActorHasTag` _hitactor "Player") _hitactor)
    (else
      (return false null))))

(fn `EndSprint`
  (set `CharacterMovementComponent.MaxWalkSpeed` (`self.WalkGroundSpeed`) (`self.CharacterMovement`))
  (set `self.IsSprint` false))

(fn `UserConstructionScript`)